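; Watergun minigame in which the player aims and fires water projectiles at a moving target to score points before a timer ends.
; Input rotates a clamped aim arrow and spawns BP_WaterProjectile at the barrel with velocity along that arrow.
; While playing, Tick moves the target within bounds and refreshes the UI, and projectile overlaps on the capsule add score.
; Named function timers periodically randomize target velocity and finish the round.
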(event `self.Capsule.OnComponentBeginOverlap`
  (params (OverlappedComponent :type "PrimitiveComponent Object Reference") (OtherActor :type "Actor Object Reference") (OtherComp :type "PrimitiveComponent Object Reference") (OtherBodyIndex :type Integer) (bFromSweep :type Boolean) (SweepResult :type "HitResult Structure (by ref)"))
  (if (and (`self.isPlaying`) (== (`GameplayStatics.GetObjectClass` OtherActor) "/Game/Game/Minigames/Watergun/BP_WaterProjectile.BP_WaterProjectile_C"))
    (set `self.Score` (+ (`self.Score`) 1))))

(event `self.ReceiveTick`
  (params (DeltaSeconds :type "Float (single-precision)"))
  (`parent.ReceiveTick` DeltaSeconds)
  (if (`self.isPlaying`)
    (`self.tickTarget` DeltaSeconds)
    (`self.updatePUI`)))

(event `EnhancedInput|/Game/Game/Input/IA_DirMove`
  (params (ActionValue :type "Vector2D Structure") (ElapsedSeconds :type "Float (double-precision)") (TriggeredSeconds :type "Float (double-precision)") (InputAction :type "InputAction Object Reference" :default "/Game/Game/Input/IA_DirMove.IA_DirMove"))
  (bind _aim_sens (`self.AIM_SENS`))
  (bind _aimarrow (`self.AimArrow`))
  (bind (_relativerotation_roll _relativerotation_pitch _relativerotation_yaw) (`KismetMathLibrary.BreakRotator` (`SceneComponent.RelativeRotation` _aimarrow)))
  (bind _returnvalue (`KismetMathLibrary.FClamp` (+ (* ActionValue_X _aim_sens) _relativerotation_yaw) -60.0 60.0))
  (bind _returnvalue_2 (`KismetMathLibrary.FClamp` (+ (* ActionValue_Y _aim_sens 1.0) _relativerotation_pitch) -20.0 60.0))
  (:`Triggered`
    (`KismetSystemLibrary.PrintString` (`KismetStringLibrary.Concat_StrStr` "AIM [ X: " (`KismetStringLibrary.Conv_DoubleToString` _returnvalue_2) " |  Y: " (`KismetStringLibrary.Conv_DoubleToString` _returnvalue) " ]") false false)
    (`SceneComponent.K2_SetRelativeRotation` _aimarrow (`KismetMathLibrary.MakeRotator` 0.0 _returnvalue_2 _returnvalue) false false)))

(event `EnhancedInput|/Game/Game/Input/IA_ActionA`
  (params (ActionValue :type Boolean) (ElapsedSeconds :type "Float (double-precision)") (TriggeredSeconds :type "Float (double-precision)") (InputAction :type "InputAction Object Reference" :default "/Game/Game/Input/IA_ActionA.IA_ActionA"))
  (:`Triggered`
    (bind _returnvalue (`|SpawnActorFromClass` "/Game/Game/Minigames/Watergun/BP_WaterProjectile.BP_WaterProjectile_C" (`KismetMathLibrary.MakeTransform` (`SceneComponent.K2_GetComponentLocation` (`self.Barrel`))) "Undefined" "MultiplyWithRoot" null null :!label _label))
    (`PrimitiveComponent.SetPhysicsLinearVelocity` (`/Game/Game/Minigames/Watergun/BP_WaterProjectile.Sphere` _returnvalue) (* (`KismetMathLibrary.GetForwardVector` (`SceneComponent.K2_GetComponentRotation` (`self.AimArrow`))) (`self.ShotPower`)) false "None"))
  (:`Started`
    (goto _label))
  (:`Ongoing`
    (goto _label)))

(fn `endTimer`
  (`self.Finish`)
  (set `self.isPlaying` false))

(fn `randomizeTargetVelo`
  (bind _returnvalue (`KismetMathLibrary.RandomBool`))
  (bind _returnvalue_2 (`KismetMathLibrary.RandomBool`))
  (bind _target_max_speed (`self.TARGET_MAX_SPEED`))
  (bind _returnvalue_3 (/ (`self.TARGET_MAX_SPEED`) 2.0))
  (bind _returnvalue_4 (- (* (`KismetMathLibrary.RandomFloat`) 2.0 _target_max_speed) _returnvalue_3))
  (bind _returnvalue_5 (- (* (`KismetMathLibrary.RandomFloat`) 2.0 _target_max_speed) _returnvalue_3))
  (`KismetSystemLibrary.PrintString` "Randomized Target Velo")
  (set `self.targetVelo` (`KismetMathLibrary.MakeVector` _returnvalue_5 _returnvalue_4))
  (if (and _returnvalue_2 _returnvalue)
    (bind _result (`/Engine/EditorBlueprintResources/StandardMacros.NegateFloat` _returnvalue_5)
      (:`  `
        (bind _result_2 (`/Engine/EditorBlueprintResources/StandardMacros.NegateFloat` _returnvalue_4)
          (:`  `
            (set `self.targetVelo` (`KismetMathLibrary.MakeVector` _result _result_2))))))
    (elif (and _returnvalue_2 (not _returnvalue))
      (bind _result_3 (`/Engine/EditorBlueprintResources/StandardMacros.NegateFloat` _returnvalue_5)
        (:`  `
          (set `self.targetVelo` (`KismetMathLibrary.MakeVector` _result_3 _returnvalue_4))))
      (elif (and (not _returnvalue_2) _returnvalue)
        (bind _result_4 (`/Engine/EditorBlueprintResources/StandardMacros.NegateFloat` _returnvalue_4)
          (:`  `
            (set `self.targetVelo` (`KismetMathLibrary.MakeVector` _returnvalue_5 _result_4))))
        (elif (and (not _returnvalue_2) (not _returnvalue))
          _
          (else
            _)))))
  (`KismetSystemLibrary.K2_SetTimer` null "randomizeTargetVelo" 2.0))

(fn `Start`
  (`parent.Start`)
  (`KismetSystemLibrary.K2_SetTimer` null "endTimer" 15.0)
  (set `self.isPlaying` true)
  (`KismetSystemLibrary.K2_SetTimer` null "randomizeTargetVelo" 3.0))

(fn `tickTarget`
  (params (deltaTime :type "Float (double-precision)"))
  (bind _target (`self.Target`))
  (bind _target_max_range (`self.TARGET_MAX_RANGE`))
  (bind (_returnvalue_x _returnvalue_y) (`KismetMathLibrary.BreakVector` (+ (* (`self.targetVelo`) deltaTime) (`SceneComponent.RelativeLocation` _target))))
  (`SceneComponent.K2_SetRelativeLocation` _target (`KismetMathLibrary.MakeVector` (`KismetMathLibrary.FClamp` _returnvalue_x (* _target_max_range -1.0) _target_max_range) (`KismetMathLibrary.FClamp` _returnvalue_y (* _target_max_range -1.0) _target_max_range) 102.0) false false))

(fn `updatePUI`
  (message `/Game/Game/Minigames/BPI_PlayerUI.updatePUI` (`self.PUI_ref`) "Aim: WASD \nShoot: R \nShoot: B Button" (`KismetSystemLibrary.K2_GetTimerRemainingTime` null "endTimer") (`self.Score`)))

(fn `UserConstructionScript`
  (`parent.UserConstructionScript`)
  (set `self.MinigameID` 4))