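; Timed basketball minigame, built on a parent minigame class, in which the player throws balls at a moving hoop to score.
; Input rotates a clamped aim arrow, adjusts throw power and launches physics projectiles along the arrow, with a cooldown between shots.
; Tick drifts the hoop within bounds at a periodically randomized velocity and updates the UI with time and score.
; Projectile overlaps with the hoop add points until the timer calls Finish.
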(event `self.ReceiveBeginPlay`)

(event `self.ReceiveTick`
  (params (DeltaSeconds :type "Float (single-precision)"))
  (if (`self.isPlaying`)
    (`self.tickTarget` DeltaSeconds)
    (`self.updatePUI`)))

(event `EnhancedInput|/Game/Game/Input/IA_ActionA`
  (params (ActionValue :type Boolean) (ElapsedSeconds :type "Float (double-precision)") (TriggeredSeconds :type "Float (double-precision)") (InputAction :type "InputAction Object Reference" :default "/Game/Game/Input/IA_ActionA.IA_ActionA"))
  (:`Started`
    (if (`self.canShoot`)
      (set `self.canShoot` false)
      (`KismetSystemLibrary.K2_SetTimer` null "shotCooldown" (`self.SHOT_COOLDOWN_TIME`))
      (bind _returnvalue (`|SpawnActorFromClass` "/Game/Game/Minigames/Basketball/BP_BasketballProjectile.BP_BasketballProjectile_C" (`KismetMathLibrary.MakeTransform` (`SceneComponent.K2_GetComponentLocation` (`self.AimArrow`))) "Undefined" "MultiplyWithRoot" null null))
      (`PrimitiveComponent.SetPhysicsLinearVelocity` (`/Game/Game/Minigames/Basketball/BP_BasketballProjectile.Sphere` _returnvalue) (* (`KismetMathLibrary.GetForwardVector` (`SceneComponent.K2_GetComponentRotation` (`self.AimArrow`))) (`self.throwPower`)) false "None"))))

(event `EnhancedInput|/Game/Game/Input/IA_DirMove`
  (params (ActionValue :type "Vector2D Structure") (ElapsedSeconds :type "Float (double-precision)") (TriggeredSeconds :type "Float (double-precision)") (InputAction :type "InputAction Object Reference" :default "/Game/Game/Input/IA_DirMove.IA_DirMove"))
  (bind _throw_aim_sens (`self.THROW_AIM_SENS`))
  (bind _aimarrow (`self.AimArrow`))
  (bind (_relativerotation_roll _relativerotation_pitch _relativerotation_yaw) (`KismetMathLibrary.BreakRotator` (`SceneComponent.RelativeRotation` _aimarrow)))
  (:`Triggered`
    (`SceneComponent.K2_SetRelativeRotation` _aimarrow (`KismetMathLibrary.MakeRotator` 0.0 (`KismetMathLibrary.FClamp` (+ (* ActionValue_Y _throw_aim_sens 1.0) _relativerotation_pitch) 20.0 75.0) (`KismetMathLibrary.FClamp` (+ (* ActionValue_X _throw_aim_sens) _relativerotation_yaw) -60.0 60.0)) false false)))

(event `EnhancedInput|/Game/Game/Input/IA_ActionB`
  (params (ActionValue :type Boolean) (ElapsedSeconds :type "Float (double-precision)") (TriggeredSeconds :type "Float (double-precision)") (InputAction :type "InputAction Object Reference" :default "/Game/Game/Input/IA_ActionB.IA_ActionB"))
  (:`Triggered`
    (set `self.throwPower` (- (`self.throwPower`) (`self.THROW_ADJUST_SENS`)) :!label _label))
  (:`Started`
    (goto _label)))

(event `EnhancedInput|/Game/Game/Input/IA_ActionC`
  (params (ActionValue :type Boolean) (ElapsedSeconds :type "Float (double-precision)") (TriggeredSeconds :type "Float (double-precision)") (InputAction :type "InputAction Object Reference" :default "/Game/Game/Input/IA_ActionC.IA_ActionC"))
  (:`Triggered`
    (set `self.throwPower` (+ (`self.throwPower`) (`self.THROW_ADJUST_SENS`)) :!label _label_2))
  (:`Started`
    (goto _label_2)))

(event `self.Hoop.OnComponentBeginOverlap`
  (params (OverlappedComponent :type "PrimitiveComponent Object Reference") (OtherActor :type "Actor Object Reference") (OtherComp :type "PrimitiveComponent Object Reference") (OtherBodyIndex :type Integer) (bFromSweep :type Boolean) (SweepResult :type "HitResult Structure (by ref)"))
  (if (and (`self.isPlaying`) (== (`GameplayStatics.GetObjectClass` OtherActor) "/Game/Game/Minigames/Basketball/BP_BasketballProjectile.BP_BasketballProjectile_C"))
    (set `self.Score` (+ (`self.Score`) 1))))

(fn `basketballTimer`
  (`self.Finish`)
  (set `self.isPlaying` false))

(fn `NewFunction_0`)

(fn `randomizeTargetVelo`
  (bind _target_max_speed (`self.TARGET_MAX_SPEED`))
  (bind _returnvalue (/ (`self.TARGET_MAX_SPEED`) 2.0))
  (`KismetSystemLibrary.PrintString` "Randomized Target Velo")
  (set `self.targetVelo` (`KismetMathLibrary.MakeVector` (- (* (`KismetMathLibrary.RandomFloat`) 2.0 _target_max_speed) _returnvalue) (- (* (`KismetMathLibrary.RandomFloat`) 2.0 _target_max_speed) _returnvalue)))
  (if (`self.isPlaying`)
    (`KismetSystemLibrary.K2_SetTimer` null "randomizeTargetVelo" 3.0)))

(fn `shotCooldown`
  (set `self.canShoot` true))

(fn `Start`
  (`parent.Start`)
  (`KismetSystemLibrary.PrintString` "Basketball")
  (`KismetSystemLibrary.K2_SetTimer` null "basketballTimer" 30.0)
  (set `self.isPlaying` true)
  (`KismetSystemLibrary.K2_SetTimer` null "randomizeTargetVelo" 3.0))

(fn `tickTarget`
  (params (deltaTime :type "Float (double-precision)"))
  (bind _hooptarget (`self.HoopTarget`))
  (bind _target_max_range (`self.TARGET_MAX_RANGE`))
  (bind (_returnvalue_x _returnvalue_y) (`KismetMathLibrary.BreakVector` (+ (* (`self.targetVelo`) deltaTime) (`SceneComponent.RelativeLocation` _hooptarget))))
  (`SceneComponent.K2_SetRelativeLocation` _hooptarget (`KismetMathLibrary.MakeVector` (`KismetMathLibrary.FClamp` _returnvalue_x (* _target_max_range -1.0) _target_max_range) (`KismetMathLibrary.FClamp` _returnvalue_y (* _target_max_range -1.0) _target_max_range)) false false))

(fn `updatePUI`
  (message `/Game/Game/Minigames/BPI_PlayerUI.updatePUI` (`self.PUI_ref`) "Aim: WASD \nShoot: R Key \nShoot: B Button" (`KismetSystemLibrary.K2_GetTimerRemainingTime` null "basketballTimer") (`self.Score`)))

(fn `UserConstructionScript`
  (`parent.UserConstructionScript`)
  (set `self.MinigameID` 1))