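; Ladder-climbing minigame where the player hits random three-button prompts while balancing a tilting ladder against a countdown.
; Correct presses raise score and character mesh, wrong ones lower them, and prompts reroll after each press or timeout.
; Each reroll resets tilt velocity to push further off-center, plus randomness scaled by score, which directional input counters.
; Tick rotates the ladder and updates the UI; excessive tilt or timer expiry ends the game.
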(event `self.ReceiveTick`
  (params (DeltaSeconds :type "Float (single-precision)"))
  (if (`self.isPlaying`)
    (`self.tickTilt` DeltaSeconds)
    (`self.updatePUI`)))

(event `EnhancedInput|/Game/Game/Input/IA_ActionA`
  (params (ActionValue :type Boolean) (ElapsedSeconds :type "Float (double-precision)") (TriggeredSeconds :type "Float (double-precision)") (InputAction :type "InputAction Object Reference" :default "/Game/Game/Input/IA_ActionA.IA_ActionA"))
  (:`Started`
    (if (== (`self.activeQTEid`) 0)
      (`self.succeedQTE`)
      (else
        (`self.failQTE`)))))

(event `EnhancedInput|/Game/Game/Input/IA_ActionB`
  (params (ActionValue :type Boolean) (ElapsedSeconds :type "Float (double-precision)") (TriggeredSeconds :type "Float (double-precision)") (InputAction :type "InputAction Object Reference" :default "/Game/Game/Input/IA_ActionB.IA_ActionB"))
  (:`Started`
    (if (== (`self.activeQTEid`) 1)
      (`self.succeedQTE`)
      (else
        (`self.failQTE`)))))

(event `EnhancedInput|/Game/Game/Input/IA_ActionC`
  (params (ActionValue :type Boolean) (ElapsedSeconds :type "Float (double-precision)") (TriggeredSeconds :type "Float (double-precision)") (InputAction :type "InputAction Object Reference" :default "/Game/Game/Input/IA_ActionC.IA_ActionC"))
  (:`Started`
    (if (== (`self.activeQTEid`) 2)
      (`self.succeedQTE`)
      (else
        (`self.failQTE`)))))

(event `EnhancedInput|/Game/Game/Input/IA_DirMove`
  (params (ActionValue :type "Vector2D Structure") (ElapsedSeconds :type "Float (double-precision)") (TriggeredSeconds :type "Float (double-precision)") (InputAction :type "InputAction Object Reference" :default "/Game/Game/Input/IA_DirMove.IA_DirMove"))
  (:`Triggered`
    (set `self.tiltVelo` (+ (* ActionValue_X (`self.MAX_TILT_ACCEL`)) (`self.tiltVelo`)))))

(fn `failQTE`
  (bind _skeletalmesh (`self.SkeletalMesh`))
  (set `self.Score` (`KismetMathLibrary.Clamp` (- (`self.Score`) 1) 0 20))
  (`KismetSystemLibrary.PrintString` "QTE Fail, Oof")
  (`self.quickTimeEvent`)
  (`SceneComponent.K2_SetRelativeLocation` _skeletalmesh (`KismetMathLibrary.MakeVector` (.x (`SceneComponent.RelativeLocation` _skeletalmesh)) (.y (`SceneComponent.RelativeLocation` _skeletalmesh)) (+ (.z (`SceneComponent.RelativeLocation` _skeletalmesh)) -3.0)) false false))

(fn `Finish`
  (`parent.Finish`)
  (set `self.isPlaying` false)
  (`SceneComponent.SetVisibility` (`self.SkeletalMesh`) false false)
  (`Widget.RemoveFromParent` (`self.Ladder_Ui`))
  (`SceneComponent.K2_SetRelativeRotation` :`self` (`self.SM_Ladder`)))

(fn `ladderTimer`
  (`self.Finish`))

(fn `quickTimeEvent`
  (bind _ladder_ui (`self.Ladder_Ui`))
  (set `self.activeQTEid` (`KismetMathLibrary.RandomInteger` 3))
  (`KismetSystemLibrary.K2_SetTimer` null "quickTimeEvent" 5.0)
  (`self.randomTiltChange`)
  (switch `int` (`self.activeQTEid`)
    (:`0`
      (`/Game/Game/LadderUi.Quick_time_update` _ladder_ui 0))
    (:`1`
      (`/Game/Game/LadderUi.Quick_time_update` _ladder_ui 1))
    (:`2`
      (`/Game/Game/LadderUi.Quick_time_update` _ladder_ui 2))))

(fn `randomTiltChange`
  (bind (_relativerotation_roll _relativerotation_pitch _relativerotation_yaw) (`KismetMathLibrary.BreakRotator` (`SceneComponent.RelativeRotation` (`self.SM_Ladder`))))
  (bind _returnvalue (* (`self.MAX_RAND_TILT`) (/ (`self.Score`) 10.0)))
  (set `self.tiltVelo` (+ (* (`KismetMathLibrary.FClamp` _relativerotation_yaw -1.0) -10.0) (- (* (`KismetMathLibrary.RandomFloat`) _returnvalue) (/ _returnvalue 2.0)))))

(fn `Start`
  (`parent.Start`)
  (`KismetSystemLibrary.K2_SetTimer` null "ladderTimer" 90.0)
  (set `self.isPlaying` true)
  (`SceneComponent.SetVisibility` (`self.SkeletalMesh`) true false)
  (bind _returnvalue (`|CreateWidget` "/Game/Game/LadderUi.LadderUi_C" (`self.ActivePlayer`)))
  (`UserWidget.AddToPlayerScreen` _returnvalue 0)
  (set `self.Ladder_Ui` _returnvalue)
  (`self.quickTimeEvent`))

(fn `succeedQTE`
  (bind _skeletalmesh (`self.SkeletalMesh`))
  (set `self.Score` (+ (`self.Score`) 1))
  (`KismetSystemLibrary.PrintString` "QTE Success, Nice!")
  (`self.quickTimeEvent`)
  (`SceneComponent.K2_SetRelativeLocation` _skeletalmesh (`KismetMathLibrary.MakeVector` (.x (`SceneComponent.RelativeLocation` _skeletalmesh)) (.y (`SceneComponent.RelativeLocation` _skeletalmesh)) (+ (.z (`SceneComponent.RelativeLocation` _skeletalmesh)) 5.0)) false false))

(fn `tickTilt`
  (params (deltaTime :type "Float (double-precision)"))
  (bind _sm_ladder (`self.SM_Ladder`))
  (bind (_relativerotation_roll _relativerotation_pitch _relativerotation_yaw) (`KismetMathLibrary.BreakRotator` (`SceneComponent.RelativeRotation` _sm_ladder)))
  (bind _returnvalue (`KismetMathLibrary.FClamp` (+ (* (`self.tiltVelo`) deltaTime -1.0) _relativerotation_yaw) -180.0 180.0))
  (`SceneComponent.K2_SetRelativeRotation` _sm_ladder (`KismetMathLibrary.MakeRotator` 0.0 0.0 _returnvalue) false false)
  (if (>= (`KismetMathLibrary.Abs` _returnvalue) 90.0)
    (`KismetSystemLibrary.PrintString` "FELL OFF LADDER")
    (`self.Finish`)))

(fn `updatePUI`
  (message `/Game/Game/Minigames/BPI_PlayerUI.updatePUI` (`self.PUI_ref`) "Tilt: A/D \nWalk: R, E, or F" (`KismetSystemLibrary.K2_GetTimerRemainingTime` null "ladderTimer") (`self.Score`)))

(fn `UserConstructionScript`
  (`parent.UserConstructionScript`)
  (set `self.MinigameID` 3))