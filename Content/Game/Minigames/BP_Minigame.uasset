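; BP_Minigame is a minigame actor that takes over a player from their character, then reports that player's score when play ends.
; Two identical swap events store player and character, blend to the minigame camera and call Start, which marks it unavailable, enables input and shows that player's GamemodeTest UI.
; Finish returns control to the character, sends Score and MinigameID to ScoreCheck, resets score, removes the UI and frees the minigame.
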(event `SwapToMinigame_1`
  (params (playerRef :type "PlayerController Object Reference") (charRef :type "/Game/Game/BP_MinigamePerson Object Reference"))
  (set `self.ActivePlayer` playerRef)
  (set `self.CharRef` charRef)
  (`ActorComponent.SetActive` (`self.Minigame_Camera`) true false)
  (`PlayerController.SetViewTargetWithBlend` (`self.ActivePlayer`) self 1.0 "VTBlend_Linear" 0.0 false)
  (`self.Start`))

(event `/Game/Game/BPI_Minigame.SwapToMinigame`
  (params (playerRef :type "PlayerController Object Reference") (charRef :type "/Game/Game/BP_MinigamePerson Object Reference"))
  (set `self.ActivePlayer` playerRef)
  (set `self.CharRef` charRef)
  (`ActorComponent.SetActive` (`self.Minigame_Camera`) true false)
  (`PlayerController.SetViewTargetWithBlend` (`self.ActivePlayer`) self 1.0 "VTBlend_Linear" 0.0 false)
  (`self.Start`))

(fn `Finish`
  (bind _score (`self.Score`))
  (`KismetSystemLibrary.PrintString` "Minigame Done")
  (`/Game/Game/BP_MinigamePerson.swapToCharacter` (`self.CharRef`) (`self.ActivePlayer`))
  (`self.DisableInput` (`self.ActivePlayer`))
  (`ActorComponent.SetActive` (`self.Minigame_Camera`) false false)
  (bind _asgamemode_test (cast `/Game/Game/GamemodeTest` (`GameplayStatics.GetGameMode`)))
  (`/Game/Game/GamemodeTest.ScoreCheck` _asgamemode_test _score (`self.ActivePlayer`) (`self.MinigameID`))
  (`KismetSystemLibrary.PrintString` (`KismetStringLibrary.Concat_StrStr` "SCORE SENT: " (`KismetStringLibrary.Conv_IntToString` _score)))
  (set `self.Score` 0)
  (bind _asgamemode_test_2 (cast `/Game/Game/GamemodeTest` (`GameplayStatics.GetGameMode`)))
  (if (== (`self.ActivePlayer`) (`/Game/Game/GamemodeTest.player1` _asgamemode_test_2))
    (`Widget.RemoveFromParent` (`/Game/Game/GamemodeTest.p1ui` _asgamemode_test_2))
    (else
      (`Widget.RemoveFromParent` (`/Game/Game/GamemodeTest.p2ui` _asgamemode_test_2))))
  (set `self.available` true))

(fn `Start`
  (set `self.available` false)
  (`EnhancedInputSubsystemInterface.AddMappingContext` (pcsubsystem `EnhancedInputLocalPlayerSubsystem` (`self.ActivePlayer`)) "/Game/Game/Input/IMC_Minigame.IMC_Minigame" 0 (struct))
  (`self.EnableInput` (`self.ActivePlayer`))
  (bind _asgamemode_test (cast `/Game/Game/GamemodeTest` (`GameplayStatics.GetGameMode`)))
  (if (== (`/Game/Game/GamemodeTest.player1` _asgamemode_test) (`self.ActivePlayer`))
    (bind _p1ui (`/Game/Game/GamemodeTest.p1ui` _asgamemode_test))
    (`UserWidget.AddToPlayerScreen` _p1ui 0)
    (set `self.PUI_ref` _p1ui)
    (else
      (bind _p2ui (`/Game/Game/GamemodeTest.p2ui` _asgamemode_test))
      (`UserWidget.AddToPlayerScreen` _p2ui 0)
      (set `self.PUI_ref` _p2ui))))

(fn `UserConstructionScript`)