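; Whack-a-mole minigame in which a player moves a hammer within a clamped range and briefly drops it to strike.
; Start sets timers to end the round and to repeatedly spawn batches of Mole_actor at random cone locations, passing each a back-reference.
; Tick pushes controls, remaining time and score to the player UI.
; After the round, the next spawn call colors a light by whether Player1 tops the GamemodeTest high scores.
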(event `self.ReceiveTick`
  (params (DeltaSeconds :type "Float (single-precision)"))
  (`parent.ReceiveTick` DeltaSeconds)
  (`self.updatePUI`))

(event `EnhancedInput|/Game/Game/Input/IA_DirMove`
  (params (ActionValue :type "Vector2D Structure") (ElapsedSeconds :type "Float (double-precision)") (TriggeredSeconds :type "Float (double-precision)") (InputAction :type "InputAction Object Reference" :default "/Game/Game/Input/IA_DirMove.IA_DirMove"))
  (bind _hammer (`self.Hammer`))
  (bind _hammer_move_speed (`self.HAMMER_MOVE_SPEED`))
  (bind _hammer_max_range (`self.HAMMER_MAX_RANGE`))
  (bind _returnvalue (* _hammer_max_range -1.0))
  (bind (_relativelocation_x _relativelocation_y) (`KismetMathLibrary.BreakVector` (`SceneComponent.RelativeLocation` _hammer)))
  (:`Triggered`
    (`SceneComponent.K2_SetRelativeLocation` _hammer (`KismetMathLibrary.MakeVector` (`KismetMathLibrary.FClamp` (+ (* ActionValue_Y _hammer_move_speed 1.0) _relativelocation_x) _returnvalue _hammer_max_range) (`KismetMathLibrary.FClamp` (+ (* ActionValue_X _hammer_move_speed) _relativelocation_y) _returnvalue _hammer_max_range)) false false)))

(event `EnhancedInput|/Game/Game/Input/IA_ActionA`
  (params (ActionValue :type Boolean) (ElapsedSeconds :type "Float (double-precision)") (TriggeredSeconds :type "Float (double-precision)") (InputAction :type "InputAction Object Reference" :default "/Game/Game/Input/IA_ActionA.IA_ActionA"))
  (bind _hammer (`self.Hammer`))
  (bind _hammer_2 (`self.Hammer`))
  (bind (_relativelocation_x _relativelocation_y) (`KismetMathLibrary.BreakVector` (`SceneComponent.RelativeLocation` _hammer)))
  (bind (_relativelocation_x_2 _relativelocation_y_2) (`KismetMathLibrary.BreakVector` (`SceneComponent.RelativeLocation` _hammer_2)))
  (:`Started`
    (`SceneComponent.K2_SetRelativeLocation` _hammer_2 (`KismetMathLibrary.MakeVector` _relativelocation_x_2 _relativelocation_y_2 -50.0) false false)
    (`KismetSystemLibrary.Delay` 0.1)
    (`SceneComponent.K2_SetRelativeLocation` _hammer (`KismetMathLibrary.MakeVector` _relativelocation_x _relativelocation_y) false false)))

(fn `activate_random`
  (for _ (range 3)
    (bind _returnvalue (`|SpawnActorFromClass` "/Game/Game/Minigames/Mole_actor.Mole_actor_C" (`KismetMathLibrary.MakeTransform` (`SceneComponent.K2_GetComponentLocation` (`KismetArrayLibrary.Array_Random` (`self.spawn`)))) "Undefined" "MultiplyWithRoot" null null))
    (set `/Game/Game/Minigames/Mole_actor.wack` self _returnvalue))
  (if (`self.running`)
    (`KismetSystemLibrary.K2_SetTimer` null "activate_random" 2.0)
    (else
      (`KismetSystemLibrary.PrintString` "bricking")
      (`self.Finish`)
      (bind _asgamemode_test (cast `/Game/Game/GamemodeTest` (`GameplayStatics.GetGameMode`))
        (:`then`
          (`KismetSystemLibrary.PrintString` "working")
          (bind (_output_highscore _output_winner) (break `/Game/Game/GameScores` (`|GetArrayItem` (`/Game/Game/GamemodeTest.HighScores` _asgamemode_test))))
          (if (== (`/Game/Game/GamemodeTest.player1` _asgamemode_test) _output_winner)
            (`LightComponent.SetLightColor` (`self.RectLight`) (struct :`G` 0.003558 :`B` 1.0 :`A` 1.0) true)
            (else
              (`LightComponent.SetLightColor` (`self.RectLight`) (struct :`R` 1.0 :`G` 0.096605 :`B` 0.043523 :`A` 1.0) true))))
        (:`CastFailed`
          (`KismetSystemLibrary.PrintString` "no working"))))))

(fn `End`
  (set `self.running` false)
  (`KismetSystemLibrary.PrintString` "end")
  (`self.Finish`))

(fn `increment score`
  (bind _result (`/Engine/EditorBlueprintResources/StandardMacros.IncrementInt` (`self.Score`))
    (:`  `
      (`KismetSystemLibrary.PrintString` (`KismetStringLibrary.Concat_StrStr` "Wack score: " (`KismetStringLibrary.Conv_IntToString` _result))))))

(fn `Start`
  (set `self.running` true)
  (`KismetSystemLibrary.PrintString` "starting")
  (`parent.Start`)
  (`KismetSystemLibrary.K2_SetTimer` null "End" 15.0)
  (`KismetSystemLibrary.K2_SetTimer` null "activate_random" 5.0))

(fn `updatePUI`
  (message `/Game/Game/Minigames/BPI_PlayerUI.updatePUI` (`self.PUI_ref`) "Aim: WASD \nHammer: R Key \nHammer: B Button" (`KismetSystemLibrary.K2_GetTimerRemainingTime` null "End") (`self.Score`)))

(fn `UserConstructionScript`
  (`parent.UserConstructionScript`)
  (set `self.spawn` (`|MakeArray` (`self.Cone`) (`self.Cone1`) (`self.Cone2`) (`self.Cone3`) (`self.Cone4`) (`self.Cone5`) (`self.Cone6`) (`self.Cone7`) (`self.Cone8`)))
  (set `self.Instructions` "wack the moles")
  (set `self.MinigameID` 2))